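; Manages a player-following trail render target for the desert slide, recording tagged actors through an orthographic base-color scene capture.
; Each tick draws a persistent material into a runtime-created target, then a draw material reading that target into the result target.
; The actor follows the player in texel-snapped steps, publishing position and offset through MPC_Capture alongside range and fade speed.
; An optional debug mesh shows the capture area on the ground below the player.
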(event `self.ReceiveBeginPlay`
  ;[1 1 1] SetUp
  (`self.SetUp`))

(event `self.ReceiveTick`
  (params (DeltaSeconds :type "Float (single-precision)"))
  (bind (_returnvalue_x _returnvalue_y _returnvalue_z) (`KismetMathLibrary.BreakVector` (`self.K2_GetActorLocation`)))
  (bind _returnvalue (`self.K2_GetActorLocation` (`GameplayStatics.GetPlayerPawn` 0)))
  (bind _returnvalue_2 (/ 1.0 (`KismetMathLibrary.Conv_IntToDouble` (`self.Resolution`))))
  (bind _returnvalue_3 (* (/ 1.0 (`KismetMathLibrary.Conv_IntToDouble` (`self.Resolution`))) (`self.TrailRange`)))
  (`|ExecutionSequence`
    (:`then_0`
      ;[1 1 1] DrawRenderTarget
      (`KismetMaterialLibrary.SetVectorParameterValue` "/Game/DynamicDesertSlide/BP/DynamicDesert/Material/MPC_Capture.MPC_Capture" "CapturePosOffset" (`KismetMathLibrary.Conv_VectorToLinearColor` (* (`KismetMathLibrary.MakeVector` (`KismetMathLibrary.Conv_IntToDouble` (`KismetMathLibrary.FFloor` (.x (/ (/ (- (`self.K2_GetActorLocation` (`GameplayStatics.GetPlayerPawn` 0)) (`self.K2_GetActorLocation`)) (`self.TrailRange`)) _returnvalue_2)))) (`KismetMathLibrary.Conv_IntToDouble` (`KismetMathLibrary.FFloor` (.y (/ (/ (- (`self.K2_GetActorLocation` (`GameplayStatics.GetPlayerPawn` 0)) (`self.K2_GetActorLocation`)) (`self.TrailRange`)) _returnvalue_2)))) (.z (/ (/ (- (`self.K2_GetActorLocation` (`GameplayStatics.GetPlayerPawn` 0)) (`self.K2_GetActorLocation`)) (`self.TrailRange`)) _returnvalue_2))) _returnvalue_2)))
      (`KismetRenderingLibrary.DrawMaterialToRenderTarget` (`self.RT_Persistent`) (`self.M_Persistent`)))
    (:`then_1`
      (`KismetRenderingLibrary.DrawMaterialToRenderTarget` (`self.RT_Result`) (`self.M_Draw_Dynamic`))
      (`self.K2_SetActorLocation` (`KismetMathLibrary.MakeVector` (.x (* (`KismetMathLibrary.MakeVector` (`KismetMathLibrary.Conv_IntToDouble` (`KismetMathLibrary.FFloor` (.x (/ (`self.K2_GetActorLocation` (`GameplayStatics.GetPlayerPawn` 0)) _returnvalue_3)))) (`KismetMathLibrary.Conv_IntToDouble` (`KismetMathLibrary.FFloor` (.y (/ (`self.K2_GetActorLocation` (`GameplayStatics.GetPlayerPawn` 0)) _returnvalue_3)))) (.z (/ (`self.K2_GetActorLocation` (`GameplayStatics.GetPlayerPawn` 0)) _returnvalue_3))) _returnvalue_3)) (.y (* (`KismetMathLibrary.MakeVector` (`KismetMathLibrary.Conv_IntToDouble` (`KismetMathLibrary.FFloor` (.x (/ (`self.K2_GetActorLocation` (`GameplayStatics.GetPlayerPawn` 0)) _returnvalue_3)))) (`KismetMathLibrary.Conv_IntToDouble` (`KismetMathLibrary.FFloor` (.y (/ (`self.K2_GetActorLocation` (`GameplayStatics.GetPlayerPawn` 0)) _returnvalue_3)))) (.z (/ (`self.K2_GetActorLocation` (`GameplayStatics.GetPlayerPawn` 0)) _returnvalue_3))) _returnvalue_3)) _returnvalue_z))
      (`KismetMaterialLibrary.SetVectorParameterValue` "/Game/DynamicDesertSlide/BP/DynamicDesert/Material/MPC_Capture.MPC_Capture" "CapturePos" (`KismetMathLibrary.Conv_VectorToLinearColor` (`self.K2_GetActorLocation`))))
    (:`then_2`
      ;[1 1 1] Debug
      (if (`self.DebugRange`)
        (bind _outhit (`KismetSystemLibrary.LineTraceSingleForObjects` _returnvalue (+ _returnvalue (0.0 0.0 -300.0)) (`|MakeArray` "ObjectTypeQuery1" :!type "EObjectTypeQuery Enum")))
        (bind (_bblockinghit _binitialoverlap _time _distance _location) (`GameplayStatics.BreakHitResult` _outhit))
        (if _bblockinghit
          (`SceneComponent.K2_SetWorldLocation` (`self. DebugCaptureSize`) _location false false)
          (`SceneComponent.SetVisibility` (`self. DebugCaptureSize`) true false))
        (else
          (`SceneComponent.SetVisibility` (`self. DebugCaptureSize`) false false))))))

(fn `SetUp`
  (bind _debugzscale (`self.DebugZScale`))
  (bind __debugcapturesize (`self. DebugCaptureSize`))
  (bind _rt_result (`self.RT_Result`))
  (bind _clear_color (`self.Clear Color`))
  (bind _sizex (`TextureRenderTarget2D.SizeX` _rt_result))
  (bind (_returnvalue_x _returnvalue_y) (`KismetMathLibrary.BreakVector` (`KismetMathLibrary.Conv_DoubleToVector` (/ (`self.TrailRange`) 100.0))))
  (`|ExecutionSequence`
    (:`then_0`
      ;[1 1 1] RenderTargetSetting
      (set `self.Resolution` _sizex)
      (bind _returnvalue (`KismetRenderingLibrary.CreateRenderTarget2D` _sizex _sizex (`TextureRenderTarget2D.RenderTargetFormat` _rt_result)))
      (set `self.RT_Persistent` _returnvalue)
      (`KismetRenderingLibrary.ClearRenderTarget2D` (`self.RT_Result`) _clear_color)
      (`KismetRenderingLibrary.ClearRenderTarget2D` (`self.RT_Persistent`) _clear_color)
      ;[1 1 1] SceneCaptureSetting
      (set `SceneCaptureComponent.CaptureSource` "SCS_BaseColor" (`self.Capture_TrailDraw`))
      (set `SceneCaptureComponent2D.ProjectionType` "Orthographic" (`self.Capture_TrailDraw`))
      (set `SceneCaptureComponent2D.OrthoWidth` (`self.TrailRange`) (`self.Capture_TrailDraw`))
      (bind _outactors (`GameplayStatics.GetAllActorsWithTag` (`self.CaptureActorTag`)))
      (set `SceneCaptureComponent.ShowOnlyActors` _outactors (`self.Capture_TrailDraw`))
      ;[1 1 1] SetMaterialParam
      (`KismetMaterialLibrary.SetVectorParameterValue` "/Game/DynamicDesertSlide/BP/DynamicDesert/Material/MPC_Capture.MPC_Capture" "CapturePos" (`KismetMathLibrary.Conv_VectorToLinearColor` (`self.K2_GetActorLocation`)))
      (`KismetMaterialLibrary.SetScalarParameterValue` "/Game/DynamicDesertSlide/BP/DynamicDesert/Material/MPC_Capture.MPC_Capture" "CaptureRange" (`self.TrailRange`))
      (`KismetMaterialLibrary.SetScalarParameterValue` "/Game/DynamicDesertSlide/BP/DynamicDesert/Material/MPC_Capture.MPC_Capture" "TrailFadeSpeed" (`self.TrailFadeSpeed`))
      (bind _returnvalue_2 (`KismetMaterialLibrary.CreateDynamicMaterialInstance` (`self.M_Draw`)))
      (bind _output_get (set `self.M_Draw_Dynamic` _returnvalue_2))
      (`MaterialInstanceDynamic.SetTextureParameterValue` _output_get "Persistent" (`self.RT_Persistent`))
      ;[1 1 1] Set Initial Position
      (`SceneComponent.K2_SetWorldLocation` (`self.Capture_TrailDraw`) (`KismetMathLibrary.MakeVector` (.x (`self.K2_GetActorLocation`)) (.y (`self.K2_GetActorLocation`)) -10000.0) false false))
    (:`then_1`
      ;[1 1 1] Debug
      (`SceneComponent.SetWorldScale3D` __debugcapturesize (`KismetMathLibrary.MakeVector` _returnvalue_x _returnvalue_y _debugzscale))
      (`SceneComponent.K2_SetRelativeLocation` __debugcapturesize (`KismetMathLibrary.MakeVector` 0.0 0.0 (* (* 50.0 _debugzscale) -1.0)) false false))))

(fn `UserConstructionScript`
  (`self.SetUp`))