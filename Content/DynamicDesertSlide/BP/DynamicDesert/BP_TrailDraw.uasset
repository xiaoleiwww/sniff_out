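; BP_TrailDraw is an actor that shows a brush component for drawing trails in the dynamic desert slide system.
; On BeginPlay it sets the player pawn as owner, hides the brush from that owner's view with Owner No See, and applies its material.
; Each Tick, a vertical line trace gates the brush, showing it only on a hit after enough 2D movement since the last stamp, otherwise hiding it.
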(event `self.ReceiveBeginPlay`
  (`self.SetUp`))

(event `self.ReceiveTick`
  (params (DeltaSeconds :type "Float (single-precision)"))
  (`self.Update Brush Visibility`))

(fn `SetUp`
  ;[1 1 1] SeeSetting
  (`self.SetOwner` (`GameplayStatics.GetPlayerPawn` 0))
  (`PrimitiveComponent.SetOwnerNoSee` (`self.Brush`) true)
  (set `self.pos` (0.0 0.0 -10000000.0))
  (`PrimitiveComponent.SetMaterial` (`self.Brush`) 0 (`self.Material`)))

(fn `Update Brush Visibility`
  (bind _returnvalue (`self.K2_GetActorLocation`))
  (bind _returnvalue_2 (`self.K2_GetActorLocation`))
  (bind _tracerange (`self.TraceRange`))
  (bind (_outhit _returnvalue_3) (`KismetSystemLibrary.LineTraceSingleForObjects` :`Start` (+ _returnvalue (`KismetMathLibrary.MakeVector` 0.0 0.0 _tracerange)) :`End` (+ _returnvalue (`KismetMathLibrary.MakeVector` 0.0 0.0 (* _tracerange -1.0))) :`ObjectTypes` (`self.TraceObjects`) :`DrawDebugType` (`self.Draw Debug Type`)))
  (if (and _returnvalue_3 (>= (`KismetMathLibrary.Vector_Distance2D` (`self.pos`) _returnvalue_2) (`self.Draw Interval Distance`)))
    (set `self.pos` _returnvalue_2)
    (`SceneComponent.SetVisibility` (`self.Brush`) true false)
    (else
      (`SceneComponent.SetVisibility` (`self.Brush`) false false))))

(fn `UserConstructionScript`)